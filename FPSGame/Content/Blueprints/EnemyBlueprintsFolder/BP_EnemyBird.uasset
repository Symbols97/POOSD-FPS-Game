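; Enemy bird (crow) pawn that chases and attacks the player, and whose death completes Level 1.
; Pawn sensing starts a chase; once chasing, Tick also issues randomly delayed moves to nearby random points, and the chase flag is never cleared.
; Attack-sphere overlap deals damage and plays an attack montage.
; Damage updates a health widget; death plays effects once, destroys the bird, then sets game mode progress flags and saves.
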(event `self.PawnSensing.OnSeePawn`
  (params (Pawn :type "Pawn Object Reference"))
  (bind _asfpscharacter (cast `FPSCharacter` Pawn))
  (`|ExecutionSequence`
    (:`then_0`
      (set `self.CanSeePlayer` true)
      (set `self.ChasingPlayer` true)
      (`|AIMoveTo` self (0.0 0.0 0.0) _asfpscharacter))
    (:`then_1`
      (`KismetSystemLibrary.RetriggerableDelay` 0.6)
      (set `self.CanSeePlayer` false))))

(event `self.ReceiveTick`
  (params (DeltaSeconds :type "Float (single-precision)"))
  (if (`self.ChasingPlayer`)
    (`KismetSystemLibrary.Delay` (`KismetMathLibrary.RandomFloatInRange` 1.0 5.0))
    (`|AIMoveTo` self (`NavigationSystemV1.K2_GetRandomReachablePointInRadius` (`self.K2_GetActorLocation`) 200.0 null null) null)))

(event `self.AttackSphere_EnemyBird.OnComponentBeginOverlap`
  (params (OverlappedComponent :type "PrimitiveComponent Object Reference") (OtherActor :type "Actor Object Reference") (OtherComp :type "PrimitiveComponent Object Reference") (OtherBodyIndex :type Integer) (bFromSweep :type Boolean) (SweepResult :type "HitResult Structure (by ref)"))
  (bind _asbp_fpscharacter (cast `/Game/Blueprints/Player/BP_FPSCharacter` OtherActor))
  (`self.enemyBirdMainAttack`)
  (`GameplayStatics.ApplyDamage` _asbp_fpscharacter 10.0)
  (`self.PlayAnimMontage` "/Game/EnemyModelsFolder/Crow/Animations/Montage_Crow_Attacks.Montage_Crow_Attacks"))

(event `self.ReceiveBeginPlay`
  (bind _asbp_enemy_health (cast `/Game/Blueprints/EnemyBlueprintsFolder/BP_EnemyHealth` (`WidgetComponent.GetUserWidgetObject` (`self.Widget`))))
  (bind _output_get (set `self.As BP Enemy Health` _asbp_enemy_health))
  (set `/Game/Blueprints/EnemyBlueprintsFolder/BP_EnemyHealth.EnemyCurrentHealth` (`self.currentHealth`) _output_get)
  (set `/Game/Blueprints/EnemyBlueprintsFolder/BP_EnemyHealth.EnemyMaxHealth` (`self.maxHealth`) _output_get))

(event `self.ReceiveAnyDamage`
  (params (Damage :type "Float (single-precision)") (DamageType :type "DamageType Object Reference") (InstigatedBy :type "Controller Object Reference") (DamageCauser :type "Actor Object Reference"))
  (bind _output_get (set `self.currentHealth` (- (`self.currentHealth`) (* Damage 1.0))))
  (`/Game/Blueprints/EnemyBlueprintsFolder/BP_EnemyHealth.Update Enemy Health` (`self.As BP Enemy Health`) (`KismetMathLibrary.FClamp` _output_get 0.0 (`self.maxHealth`)))
  (if (<= (`self.currentHealth`) 0.0)
    (`/Engine/EditorBlueprintResources/StandardMacros.DoOnce` false
      (:`Completed`
        (`GameplayStatics.SpawnEmitterAttached` null)
        (`SkeletalMeshComponent.PlayAnimation` (`self.Mesh`) "/Game/EnemyModelsFolder/Crow/Animations/ANIM_Crow_DeathHitTheGround.ANIM_Crow_DeathHitTheGround" false)
        (`KismetSystemLibrary.Delay` 2.0)
        (`self.K2_DestroyActor`)
        (bind _asfpsgame_mode (cast `/Game/Blueprints/GameModeBase/FPSGameMode` (`GameplayStatics.GetGameMode`)))
        (set `/Game/Blueprints/GameModeBase/FPSGameMode.showPig` true _asfpsgame_mode)
        (set `/Game/Blueprints/GameModeBase/FPSGameMode.completedLevel1` true _asfpsgame_mode)
        (`/Game/Blueprints/GameModeBase/FPSGameMode.saveGame` _asfpsgame_mode)))))

(fn `UserConstructionScript`)