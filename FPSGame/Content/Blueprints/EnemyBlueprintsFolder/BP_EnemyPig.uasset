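; BP_EnemyPig is a pig enemy that wanders, chases the player on sight and deals contact damage.
; Tick issues randomly delayed moves to nearby reachable points until pawn sensing sets ChasingPlayer, which is never cleared; CanSeePlayer lapses via retriggerable delay.
; Attack sphere overlap triggers the main attack and damage.
; Incoming damage updates a health widget; at zero, an emitter and death animation precede delayed destruction.
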(event `self.PawnSensing.OnSeePawn`
  (params (Pawn :type "Pawn Object Reference"))
  (bind _asfpscharacter (cast `FPSCharacter` Pawn))
  (`|ExecutionSequence`
    (:`then_0`
      (set `self.CanSeePlayer` true)
      (set `self.ChasingPlayer` true)
      (`|AIMoveTo` self (0.0 0.0 0.0) _asfpscharacter))
    (:`then_1`
      (`KismetSystemLibrary.RetriggerableDelay` 0.6)
      (set `self.CanSeePlayer` false))))

(event `self.ReceiveTick`
  (params (DeltaSeconds :type "Float (single-precision)"))
  (if (not (`self.ChasingPlayer`))
    (`KismetSystemLibrary.Delay` (`KismetMathLibrary.RandomFloatInRange` 1.0 5.0))
    (`|AIMoveTo` self (`NavigationSystemV1.K2_GetRandomReachablePointInRadius` (`self.K2_GetActorLocation`) 200.0 null null) null)))

(event `self.AttackSphere_EnemyPig.OnComponentBeginOverlap`
  (params (OverlappedComponent :type "PrimitiveComponent Object Reference") (OtherActor :type "Actor Object Reference") (OtherComp :type "PrimitiveComponent Object Reference") (OtherBodyIndex :type Integer) (bFromSweep :type Boolean) (SweepResult :type "HitResult Structure (by ref)"))
  (bind _asbp_fpscharacter (cast `/Game/Blueprints/Player/BP_FPSCharacter` OtherActor))
  (`self.enemyPigMainAttack`)
  (`GameplayStatics.ApplyDamage` _asbp_fpscharacter 10.0))

(event `self.ReceiveBeginPlay`
  (bind _asbp_enemy_health (cast `/Game/Blueprints/EnemyBlueprintsFolder/BP_EnemyHealth` (`WidgetComponent.GetUserWidgetObject` (`self.Widget`))))
  (bind _output_get (set `self.As BP Enemy Health` _asbp_enemy_health))
  (set `/Game/Blueprints/EnemyBlueprintsFolder/BP_EnemyHealth.EnemyCurrentHealth` (`self.PigCurrentHealth`) _output_get)
  (set `/Game/Blueprints/EnemyBlueprintsFolder/BP_EnemyHealth.EnemytMaxHealth` (`self.PigMaxHealth`) _output_get))

(event `self.ReceiveAnyDamage`
  (params (Damage :type "Float (single-precision)") (DamageType :type "DamageType Object Reference") (InstigatedBy :type "Controller Object Reference") (DamageCauser :type "Actor Object Reference"))
  (bind _output_get (set `self.PigCurrentHealth` (- (`self.PigCurrentHealth`) (* Damage 1.0))))
  (`/Game/Blueprints/EnemyBlueprintsFolder/BP_EnemyHealth.Update Enemy Health` (`self.As BP Enemy Health`) (`KismetMathLibrary.FClamp` _output_get 0.0 (`self.PigMaxHealth`)))
  (if (<= (`self.PigCurrentHealth`) 0.0)
    (`GameplayStatics.SpawnEmitterAttached` null)
    (`SkeletalMeshComponent.PlayAnimation` (`self.Mesh`) "/Game/EnemyModelsFolder/Pig/Animations/ANIM_Pig_Death.ANIM_Pig_Death" false)
    (`KismetSystemLibrary.Delay` 2.0)
    (`self.K2_DestroyActor`)))

(fn `UserConstructionScript`)