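; Enemy hamster AI pawn that wanders randomly and chases the player on sight.
; Pawn sensing moves it toward the seen player and sets chase flags, which a retriggerable delay clears shortly after sightings stop.
; While not chasing, Tick issues moves to random reachable nearby points after random delays.
; An attack sphere overlapping the player character calls the main attack implemented in C++.
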(event `self.PawnSensing.OnSeePawn`
  (params (Pawn :type "Pawn Object Reference"))
  (bind _asfpscharacter (cast `FPSCharacter` Pawn))
  (`|ExecutionSequence`
    (:`then_0`
      (set `self.canSeePlayer` true)
      (set `self.chasingPlayer` true)
      (`|AIMoveTo` self (0.0 0.0 0.0) _asfpscharacter))
    (:`then_1`
      (`KismetSystemLibrary.RetriggerableDelay` 0.6)
      (set `self.canSeePlayer` false)
      (set `self.chasingPlayer` false))))

(event `self.ReceiveTick`
  (params (DeltaSeconds :type "Float (single-precision)"))
  (if (not (`self.chasingPlayer`))
    (`KismetSystemLibrary.Delay` (`KismetMathLibrary.RandomFloatInRange` 1.0 5.0))
    (`|AIMoveTo` self (`NavigationSystemV1.K2_GetRandomReachablePointInRadius` (`self.K2_GetActorLocation`) 900.0 null null) null)))

(event `self.AttackSphere_EnemyHamster.OnComponentBeginOverlap`
  (params (OverlappedComponent :type "PrimitiveComponent Object Reference") (OtherActor :type "Actor Object Reference") (OtherComp :type "PrimitiveComponent Object Reference") (OtherBodyIndex :type Integer) (bFromSweep :type Boolean) (SweepResult :type "HitResult Structure (by ref)"))
  (cast `/Game/Blueprints/Player/BP_FPSCharacter` OtherActor) ; Can be replaced by DoesImplementInterface if the FPSCharacter implements an interface
  (`self.enemyHamsterMainAttack`) ; This function is in EnemyHamster c++
)

(fn `UserConstructionScript`)