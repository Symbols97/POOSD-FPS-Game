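; FPSGameMode is a game mode Blueprint that saves and loads player progress.
; SaveGame copies the show flags for hamster, pig and crow and the completion flags for three levels into a new MySaveGame object, then writes it to a single slot.
; LoadGame restores those variables when the slot exists, and both functions print debug status.
; The event graph holds no active logic, so other Blueprints must call these functions.
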(fn `loadGame`
  (bind _save_slot_1 (`self.Save Slot 1`))
  (bind _returnvalue (`GameplayStatics.DoesSaveGameExist` _save_slot_1))
  (if _returnvalue
    (bind _returnvalue_2 (`GameplayStatics.LoadGameFromSlot` _save_slot_1))
    (bind _asmy_save_game (cast `/Game/Blueprints/GameModeBase/MySaveGame` _returnvalue_2))
    (set `self.showHamster` (`/Game/Blueprints/GameModeBase/MySaveGame.saved_showHamster` _asmy_save_game))
    (set `self.showPig` (`/Game/Blueprints/GameModeBase/MySaveGame.saved_showPig` _asmy_save_game))
    (set `self.showCrow` (`/Game/Blueprints/GameModeBase/MySaveGame.saved_showCrow` _asmy_save_game))
    (set `self.completedLevel1` (`/Game/Blueprints/GameModeBase/MySaveGame.saved_completedLevel1` _asmy_save_game))
    (set `self.completedLevel2` (`/Game/Blueprints/GameModeBase/MySaveGame.saved_completedLevel2` _asmy_save_game))
    (set `self.completedLevel3` (`/Game/Blueprints/GameModeBase/MySaveGame.saved_completedLevel3` _asmy_save_game))
    (`KismetSystemLibrary.PrintString` "loaded")
    (else
      (`KismetSystemLibrary.PrintString` "no game save"))))

(fn `saveGame`
  (bind _returnvalue (`GameplayStatics.CreateSaveGameObject` "/Game/Blueprints/GameModeBase/MySaveGame.MySaveGame_C"))
  (set `/Game/Blueprints/GameModeBase/MySaveGame.saved_showHamster` (`self.showHamster`) _returnvalue)
  (set `/Game/Blueprints/GameModeBase/MySaveGame.saved_showPig` (`self.showPig`) _returnvalue)
  (set `/Game/Blueprints/GameModeBase/MySaveGame.saved_showCrow` (`self.showCrow`) _returnvalue)
  (set `/Game/Blueprints/GameModeBase/MySaveGame.saved_completedLevel1` (`self.completedLevel1`) _returnvalue)
  (set `/Game/Blueprints/GameModeBase/MySaveGame.saved_completedLevel2` (`self.completedLevel2`) _returnvalue)
  (set `/Game/Blueprints/GameModeBase/MySaveGame.saved_completedLevel3` (`self.completedLevel3`) _returnvalue)
  (bind _returnvalue_2 (`GameplayStatics.SaveGameToSlot` _returnvalue (`self.Save Slot 1`)))
  (`KismetSystemLibrary.PrintString` "saved" _returnvalue_2))

(fn `UserConstructionScript`)