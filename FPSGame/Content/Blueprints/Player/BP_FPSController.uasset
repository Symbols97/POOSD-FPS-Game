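; BP_FPSController is the FPS player controller that owns the HUD and the pause menu.
; BeginPlay creates the HUD widget, and the UpdateHealth event forwards current and max health to it.
; Escape or 1 toggles pause, adding or removing a freshly created menu and switching cursor visibility and input mode.
; The UpdateHudHealth function only calls UpdateHealth with zero values.
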(event `UpdateHealth`
  (params (CurrentHealth :type "Float (double-precision)") (MaxHealth :type "Float (double-precision)"))
  (`/Game/Blueprints/UI/HUD.SetHealth` (`self.HUD`) CurrentHealth MaxHealth))

(event `self.ReceiveBeginPlay`
  (bind _returnvalue (`|CreateWidget` "/Game/Blueprints/UI/HUD.HUD_C"))
  (bind _output_get (set `self.HUD` _returnvalue))
  (`UserWidget.AddToViewport` _output_get 0))

(event `Key|Escape` :paused true
  (params (Key :type "Key Structure"))
  (bind _returnvalue (`GameplayStatics.GetPlayerController` 0))
  (:`Pressed`
    (if (`GameplayStatics.IsGamePaused`) :!label _label
      (`Widget.RemoveFromParent` (stale _returnvalue_2))
      (`GameplayStatics.SetGamePaused` false)
      (set `PlayerController.bShowMouseCursor` false _returnvalue)
      (`WidgetBlueprintLibrary.SetInputMode_GameOnly` _returnvalue)
      (else
        (bind _returnvalue_2 (`|CreateWidget` "/Game/Blueprints/UI/pauseMenu.pauseMenu_C"))
        (`UserWidget.AddToViewport` _returnvalue_2 0)
        (`GameplayStatics.SetGamePaused` true)
        (set `PlayerController.bShowMouseCursor` true _returnvalue)
        (`WidgetBlueprintLibrary.SetInputMode_GameAndUIEx` _returnvalue _returnvalue_2 "LockOnCapture" false)
        (`GameplayStatics.SetViewportMouseCaptureMode` "CapturePermanently_IncludingInitialMouseDown")))))

(event `Key|One` :paused true
  (params (Key :type "Key Structure"))
  (:`Pressed`
    (goto _label)))

(fn `updateHudHealth`
  (`self.UpdateHealth` 0.0))

(fn `UserConstructionScript`)