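; Music manager Blueprint that plays background tracks and switches between them.
; On BeginPlay it creates a 2D sound for every track in the list, starts them all together silently, then raises the initial track to the set volume.
; ChangeMusic mutes the current track and unmutes the chosen one, so switches are instant cuts between simultaneously running tracks, with no restart or crossfade.
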(event `self.ReceiveBeginPlay`
  (bind _output (`|GetArrayItem` (`self.MusicReferences`) (`self.IndexSong`)))
  (for _array_element (`self.TrackList`)
    (bind _returnvalue (`GameplayStatics.CreateSound2D` _array_element 1.0 1.0 0.0 null))
    (`KismetArrayLibrary.Array_Add` (`self.MusicReferences`) _returnvalue)
    (`AudioComponent.SetVolumeMultiplier` _returnvalue 0.0)
    (`AudioComponent.Play` _returnvalue 0.0))
  (`AudioComponent.SetVolumeMultiplier` _output (`self.Volume`))
  (set `self.CurrentSong` _output))

(event `ChangeMusic`
  (params (Index :type Integer))
  (bind _output (`|GetArrayItem` (`self.MusicReferences`) Index))
  (`AudioComponent.SetVolumeMultiplier` (`self.CurrentSong`) 0.0)
  (`AudioComponent.SetVolumeMultiplier` _output (`self.Volume`))
  (set `self.CurrentSong` _output))

(fn `UserConstructionScript`)