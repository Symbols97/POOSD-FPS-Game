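; BP_LevelBoard is an interactable board prop that opens the level selection menu.
; When interacted with, it creates a LevelSelect widget, adds it to the viewport, shows the mouse cursor and switches input to Game and UI with permanent mouse capture.
; It supplies "Level Select" as its interaction text, attached to the board component.
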(event `/Game/Weapons/Backend/InteractionInterface.OnInteracted`
  (params (Player :type "/Game/Blueprints/Player/BP_FPSCharacter Object Reference"))
  (bind _returnvalue (`GameplayStatics.GetPlayerController` 0))
  (bind _returnvalue_2 (`|CreateWidget` "/Game/Blueprints/UI/LevelSelect.LevelSelect_C"))
  (`UserWidget.AddToViewport` _returnvalue_2 0)
  (set `PlayerController.bShowMouseCursor` true _returnvalue)
  (`WidgetBlueprintLibrary.SetInputMode_GameAndUIEx` _returnvalue null "LockOnCapture" false)
  (`GameplayStatics.SetViewportMouseCaptureMode` "CapturePermanently_IncludingInitialMouseDown"))

(fn `GetInteractionText`
  (returns (Text :type Text))
  (return "Level Select"))

(fn `GetInteractionTextAttach`
  (returns (AttachComponent :type "SceneComponent Object Reference"))
  (return (`self.SM_PROP_board_01`)))

(fn `UserConstructionScript`
  (`parent.UserConstructionScript`))