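; Base weapon Blueprint that acts as an interactable "Pick Up" with its prompt attached to the skeletal mesh.
; Interacting spawns a new copy of the same class at the player, passes it to PickUpWeapon and sets it to Equipped, leaving the original in place.
; SetWeaponState disables sphere and mesh collision and resets the mesh transform when Equipped, or destroys the actor when Dropped.
; Fire is an empty stub.
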(event `/Game/Weapons/Backend/InteractionInterface.OnInteracted`
  (params (Player :type "/Game/Blueprints/Player/BP_FPSCharacter Object Reference"))
  (bind _returnvalue (`|SpawnActorFromClass` (`GameplayStatics.GetObjectClass` self) (`self.GetTransform` Player) "AlwaysSpawn" "OverrideRootScale" null null))
  (`/Game/Blueprints/Player/BP_FPSCharacter.PickUpWeapon` Player _returnvalue)
  (`self.SetWeaponState` _returnvalue "NewEnumerator1"))

(fn `Fire`
  (params (PlayerCam :type "CameraComponent Object Reference")))

(fn `GetInteractionText`
  (returns (Text :type Text))
  (return "Pick Up"))

(fn `GetInteractionTextAttach`
  (returns (AttachComponent :type "SceneComponent Object Reference"))
  (return (`self.SkeletalMesh`)))

(fn `SetWeaponState`
  (params (GunState :type "/Game/Weapons/Backend/EWeaponState Enum" :default "NewEnumerator0"))
  (bind _skeletalmesh (`self.SkeletalMesh`))
  (bind _output_get (set `self.Weapon State` GunState))
  (switch `/Game/Weapons/Backend/EWeaponState` _output_get
    (:`NewEnumerator0`
      (`self.K2_DestroyActor`))
    (:`NewEnumerator1`
      (`PrimitiveComponent.SetCollisionProfileName` (`self.Sphere`) "NoCollision" true)
      (`PrimitiveComponent.SetCollisionProfileName` _skeletalmesh "NoCollision" true)
      (`SceneComponent.ResetRelativeTransform` _skeletalmesh))))

(fn `UserConstructionScript`
  (`parent.UserConstructionScript`))